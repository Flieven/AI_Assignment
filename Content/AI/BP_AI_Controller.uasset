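; AI controller for enemies that runs the BT_Enemy behavior tree on possess.
; When AI perception successfully senses an actor whose class is exactly FirstPersonCharacter, it sets the HasLineOfSight blackboard flag and stores that actor as TargetActor.
; Neither key is cleared here when the stimulus is lost.
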(event OnTargetPerceptionUpdated(AIPerception)
  (params (Actor :type Actor%20Object%20Reference) (Stimulus :type AI%20Stimulus%20Structure))
  (Variables|Default|SetPerceivedActor Actor)
  (if (and (Utilities|Struct|BreakAIStimulus Stimulus) (== (Utilities|GetClass Actor) "/Game/FirstPersonBP/Blueprints/FirstPersonCharacter.FirstPersonCharacter_C"))
    (CallFunction|UpdateSight true)
    (CallFunction|UpdateTarget (Variables|Default|GetPerceivedActor))))

(event EventPossess
  (params (PossessedPawn :type Pawn%20Object%20Reference))
  (AI|RunBehaviorTree "/Game/AI/BT_Enemy.BT_Enemy"))

(fn ConstructionScript)

(fn UpdateSight
  (params (HasLineOfSight :type Boolean))
  (AI|Components|Blackboard|SetValueasBool (Variables|Default|GetBlackboard) (Utilities|Name|MakeLiteralName "HasLineOfSight") HasLineOfSight))

(fn UpdateTarget
  (params (Target :type Actor%20Object%20Reference))
  (AI|Components|Blackboard|SetValueasObject (Variables|Default|GetBlackboard) (Utilities|Name|MakeLiteralName "TargetActor") Target))